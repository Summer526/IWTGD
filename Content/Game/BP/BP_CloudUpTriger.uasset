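; BP_CloudUpTriger is an actor with cloud barriers that open for BP_Player through two overlap volumes.
; The Pass volume makes Cloud ignore the Pawn channel, restoring Block on exit while the stored player is valid.
; The Triger volume makes Cloud1 ignore all collision and swaps its material to the passable look.
; Any Triger end overlap restores collision and material after an Opentime delay.
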(event `self.Pass.OnComponentBeginOverlap`
  (params (OverlappedComponent :type "PrimitiveComponent Object Reference") (OtherActor :type "Actor Object Reference") (OtherComp :type "PrimitiveComponent Object Reference") (OtherBodyIndex :type Integer) (bFromSweep :type Boolean) (SweepResult :type "HitResult Structure (by ref)"))
  (bind _asbp_player (cast `/Game/Game/Characters/Player/BP_Player` OtherActor))
  (set `self.Player` _asbp_player)
  (`PrimitiveComponent.SetCollisionResponseToChannel` (`self.Cloud`) "ECC_Pawn" "ECR_Ignore"))

(event `self.Pass.OnComponentEndOverlap`
  (params (OverlappedComponent :type "PrimitiveComponent Object Reference") (OtherActor :type "Actor Object Reference") (OtherComp :type "PrimitiveComponent Object Reference") (OtherBodyIndex :type Integer))
  (`/Engine/EditorBlueprintResources/StandardMacros.IsValid` (`self.Player`)
    (:`Is Valid`
      (`PrimitiveComponent.SetCollisionResponseToChannel` (`self.Cloud`) "ECC_Pawn" "ECR_Block")
      (set `self.Player` null))))

(event `self.Triger.OnComponentBeginOverlap`
  (params (OverlappedComponent :type "PrimitiveComponent Object Reference") (OtherActor :type "Actor Object Reference") (OtherComp :type "PrimitiveComponent Object Reference") (OtherBodyIndex :type Integer) (bFromSweep :type Boolean) (SweepResult :type "HitResult Structure (by ref)"))
  (bind _cloud1 (`self.Cloud1`))
  (bind _asbp_player (cast `/Game/Game/Characters/Player/BP_Player` OtherActor))
  (set `self.Player` _asbp_player)
  (`PrimitiveComponent.SetCollisionResponseToAllChannels` _cloud1 "ECR_Ignore")
  (`PrimitiveComponent.SetMaterial` _cloud1 0 "/Game/Game/Mat/M_CloudWallPass.M_CloudWallPass"))

(event `self.Triger.OnComponentEndOverlap`
  (params (OverlappedComponent :type "PrimitiveComponent Object Reference") (OtherActor :type "Actor Object Reference") (OtherComp :type "PrimitiveComponent Object Reference") (OtherBodyIndex :type Integer))
  (bind _cloud1 (`self.Cloud1`))
  (`KismetSystemLibrary.Delay` (`self.opentime`))
  (`PrimitiveComponent.SetCollisionResponseToAllChannels` _cloud1 "ECR_Block")
  (`PrimitiveComponent.SetMaterial` _cloud1 0 "/Game/Game/Mat/M_CloudWall.M_CloudWall")
  (set `self.Player` null))

(fn `UserConstructionScript`)
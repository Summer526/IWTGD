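; Cloud actor that blinks between solid and passable on a timer, swapping its collision response and material together.
; BeginPlay makes it passable, waits an optional FirstDelay, then a FlipFlop alternates BlinkOff and BlinkOn, which re-enter it through Blink to loop.
; TimeCan and TimeCant time the switches.
; An older Tick-driven cycle remains behind DelayFinished, which is only set in unconnected nodes.
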(event `self.ReceiveTick`
  (params (DeltaSeconds :type "Float (single-precision)"))
  (bind _cloud (`self.Cloud`))
  (bind _cloud_2 (`self.Cloud`))
  (if (`self.DelayFinished`)
    (`KismetSystemLibrary.Delay` (`self.TimeCan`))
    (`PrimitiveComponent.SetCollisionResponseToAllChannels` _cloud "ECR_Block")
    (`PrimitiveComponent.SetMaterial` _cloud 0 "/Game/Game/Mat/M_CloudBlink.M_CloudBlink")
    (set `self.Player` null)
    (`KismetSystemLibrary.Delay` (`self.TimeCan't`))
    (`PrimitiveComponent.SetCollisionResponseToAllChannels` _cloud_2 "ECR_Ignore")
    (`PrimitiveComponent.SetMaterial` _cloud_2 0 "/Game/Game/Mat/M_CloudWallPass.M_CloudWallPass")
    (set `self.Player` null)))

(event `self.ReceiveBeginPlay`
  (bind _firstdelay (`self.FirstDelay`))
  (`PrimitiveComponent.SetCollisionResponseToAllChannels` (`self.Cloud`) "ECR_Ignore")
  (if (> _firstdelay 0.0)
    (`KismetSystemLibrary.Delay` _firstdelay))
  (`/Engine/EditorBlueprintResources/StandardMacros.FlipFlop` :!label _label
    (:`A`
      (`self.BlinkOff`))
    (:`B`
      (`self.BlinkOn`))))

(event `Blink`
  (goto _label))

(event `BlinkOff`
  (bind _cloud (`self.Cloud`))
  (`KismetSystemLibrary.Delay` (`self.TimeCan`))
  (`PrimitiveComponent.SetMaterial` _cloud 0 "/Game/Game/Mat/M_CloudWallPass.M_CloudWallPass")
  (`PrimitiveComponent.SetCollisionResponseToAllChannels` _cloud "ECR_Ignore")
  (`self.Blink` :!label _label_2))

(event `BlinkOn`
  (bind _cloud (`self.Cloud`))
  (`KismetSystemLibrary.Delay` (`self.TimeCan't`))
  (`PrimitiveComponent.SetCollisionResponseToAllChannels` _cloud "ECR_Block")
  (`PrimitiveComponent.SetMaterial` _cloud 0 "/Game/Game/Mat/M_CloudBlink.M_CloudBlink")
  (goto _label_2))

(fn `UserConstructionScript`)
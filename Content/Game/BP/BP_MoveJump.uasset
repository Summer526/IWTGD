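; BP_MoveJump is a moving jump pad that shuttles back and forth and launches BP_Player upward on contact.
; Construction stores the start location, and BeginPlay enables movement after an optional delay.
; Tick advances a speed-based Progress and passes it to Move, which lerps between the endpoints, pauses, then flips direction.
; Overlapping the Up component launches the player with a fixed vertical velocity and plays a jump-pad sound.
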(event `self.ReceiveBeginPlay`
  (if (> (`self.Delay`) 0.0)
    (`KismetSystemLibrary.Delay` (`self.Delay`)))
  (set `self.CanMove` true))

(event `self.ReceiveTick`
  (params (DeltaSeconds :type "Float (single-precision)"))
  (bind _startloc (`self.StartLoc`))
  (bind _returnvalue (+ _startloc (`self.Distance`)))
  (if (`self.CanMove`)
    (set `self.ProgressSpeed` (* DeltaSeconds (/ 1.0 (/ (`KismetMathLibrary.VSize` (`self.Distance`)) (`self.Speed`)))))
    (set `self.Progress` (`KismetMathLibrary.FClamp` (+ (`self.Progress`) (`self.ProgressSpeed`))))
    (switch `/Game/Game/BP/E_MoveState` (`self.MoveState`)
      (:`NewEnumerator0`
        (`self.Move` _startloc _returnvalue "NewEnumerator1"))
      (:`NewEnumerator1`
        (`self.Move` _returnvalue _startloc)))))

(event `self.Up.OnComponentBeginOverlap`
  (params (OverlappedComponent :type "PrimitiveComponent Object Reference") (OtherActor :type "Actor Object Reference") (OtherComp :type "PrimitiveComponent Object Reference") (OtherBodyIndex :type Integer) (bFromSweep :type Boolean) (SweepResult :type "HitResult Structure (by ref)"))
  (bind _asbp_player (cast `/Game/Game/Characters/Player/BP_Player` OtherActor))
  (`Character.LaunchCharacter` _asbp_player (0.0 0.0 5000.0) false true)
  (`GameplayStatics.PlaySound2D` "/Game/Game/Sound/SFX/SC_JumpPad.SC_JumpPad" 1.0 1.0 0.0 null null))

(fn `UserConstructionScript`
  (set `self.StartLoc` (`self.K2_GetActorLocation`)))
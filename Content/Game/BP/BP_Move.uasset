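; BP_Move is an actor that shuttles back and forth between its placed location and an offset set by Distance.
; The construction script records the start location, and BeginPlay enables movement after an optional Delay.
; Tick advances a clamped Progress from Speed and the distance's length, switching on MoveState between forward and reverse.
; The Move graph lerps the location without sweep, then waits for Pause at each end before flipping state.
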(event `self.ReceiveBeginPlay`
  (if (> (`self.Delay`) 0.0)
    (`KismetSystemLibrary.Delay` (`self.Delay`)))
  (set `self.CanMove` true))

(event `self.ReceiveTick`
  (params (DeltaSeconds :type "Float (single-precision)"))
  (bind _startloc (`self.StartLoc`))
  (bind _returnvalue (+ _startloc (`self.Distance`)))
  (if (`self.CanMove`)
    (set `self.ProgressSpeed` (* DeltaSeconds (/ 1.0 (/ (`KismetMathLibrary.VSize` (`self.Distance`)) (`self.Speed`)))))
    (set `self.Progress` (`KismetMathLibrary.FClamp` (+ (`self.Progress`) (`self.ProgressSpeed`))))
    (switch `/Game/Game/BP/E_MoveState` (`self.MoveState`)
      (:`NewEnumerator0`
        (`self.Move` _startloc _returnvalue "NewEnumerator1"))
      (:`NewEnumerator1`
        (`self.Move` _returnvalue _startloc)))))

(fn `UserConstructionScript`
  (set `self.StartLoc` (`self.K2_GetActorLocation`)))
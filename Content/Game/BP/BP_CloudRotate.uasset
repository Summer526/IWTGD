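; Blueprint that keeps a Cloud component slowly or steadily rolling, judging by its name and logic as a rotating cloud.
; Tick runs a single-pass loop into a Delay of Time, so rotation advances in timed steps rather than scaling by delta seconds.
; Each step adds Rotator to the component's relative roll, zeroes pitch and yaw, and keeps its relative location.
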(event `self.ReceiveBeginPlay`)

(event `self.ReceiveTick`
  (params (DeltaSeconds :type "Float (single-precision)"))
  (bind _cloud (`self.Cloud`))
  (for _ (range 1)
    (`KismetSystemLibrary.Delay` (`self.time`))
    (`SceneComponent.K2_SetRelativeLocationAndRotation` _cloud (`SceneComponent.RelativeLocation` _cloud) (`KismetMathLibrary.MakeRotator` (+ (.roll (`SceneComponent.RelativeRotation` _cloud)) (`self.rotator`))) false false)))

(fn `UserConstructionScript`)
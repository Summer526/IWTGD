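; BP_MoveCloud is a cloud actor that shuttles back and forth between its placed location and a Distance offset.
; After an optional start delay, Tick advances Progress at constant Speed and the Move macro lerps the position, pausing at each end before flipping MoveState.
; While BP_Player overlaps the Pass volume, the Cloud component ignores the Pawn channel so the player can pass through, then blocks again on exit.
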(event `self.ReceiveBeginPlay`
  (if (> (`self.Delay`) 0.0)
    (`KismetSystemLibrary.Delay` (`self.Delay`)))
  (set `self.CanMove` true))

(event `self.ReceiveTick`
  (params (DeltaSeconds :type "Float (single-precision)"))
  (bind _startloc (`self.StartLoc`))
  (bind _returnvalue (+ _startloc (`self.Distance`)))
  (if (`self.CanMove`)
    (set `self.ProgressSpeed` (* DeltaSeconds (/ 1.0 (/ (`KismetMathLibrary.VSize` (`self.Distance`)) (`self.Speed`)))))
    (set `self.Progress` (`KismetMathLibrary.FClamp` (+ (`self.Progress`) (`self.ProgressSpeed`))))
    (switch `/Game/Game/BP/E_MoveState` (`self.MoveState`)
      (:`NewEnumerator0`
        (`self.Move` _startloc _returnvalue "NewEnumerator1"))
      (:`NewEnumerator1`
        (`self.Move` _returnvalue _startloc)))))

(event `self.Pass.OnComponentBeginOverlap`
  (params (OverlappedComponent :type "PrimitiveComponent Object Reference") (OtherActor :type "Actor Object Reference") (OtherComp :type "PrimitiveComponent Object Reference") (OtherBodyIndex :type Integer) (bFromSweep :type Boolean) (SweepResult :type "HitResult Structure (by ref)"))
  (bind _asbp_player (cast `/Game/Game/Characters/Player/BP_Player` OtherActor))
  (set `self.Player` _asbp_player)
  (`PrimitiveComponent.SetCollisionResponseToChannel` (`self.Cloud`) "ECC_Pawn" "ECR_Ignore"))

(event `self.Pass.OnComponentEndOverlap`
  (params (OverlappedComponent :type "PrimitiveComponent Object Reference") (OtherActor :type "Actor Object Reference") (OtherComp :type "PrimitiveComponent Object Reference") (OtherBodyIndex :type Integer))
  (`/Engine/EditorBlueprintResources/StandardMacros.IsValid` (`self.Player`)
    (:`Is Valid`
      (`PrimitiveComponent.SetCollisionResponseToChannel` (`self.Cloud`) "ECC_Pawn" "ECR_Block")
      (set `self.Player` null))))

(fn `UserConstructionScript`
  (set `self.StartLoc` (`self.K2_GetActorLocation`)))